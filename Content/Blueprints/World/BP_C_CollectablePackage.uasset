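; Collectable package Blueprint that turns in quarter-turn yaw steps when interacted with.
; Interact advances a wrapping four-step index, then the RotationSpeed timeline lerps the ScaleScene component's relative yaw from its current rotation to the new angle.
; An IsRotating flag, set during timeline updates and cleared on finish, ignores interaction mid-turn.
; The construction script calls the parent's and sets the ID to "Package".
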(event EventInteract
  (params (Sender :type Actor%20Object%20Reference))
  (if (not (Variables|Default|GetIsRotating))
    (Variables|Default|SetStartRotation (Variables|/Script/Engine.SceneComponent|GetRelativeRotation (Variables|Default|GetScaleScene)))
    (bind _output_get (Variables|Default|SetRotationIndex (Math|Integer|%(Integer) (+ (Variables|Default|GetRotationIndex) 1) 4)))
    (Variables|Default|SetTargetRotation (Math|Rotator|MakeRotator 0.0 0.0 (Math|Conversions|ToFloat(Integer) (* _output_get 90))))
    (bind _rotationspeed (Timeline|RotationSpeed PlayFromStart)
      (:Update
        (Variables|Default|SetIsRotating true)
        (Transformation|SetRelativeRotation (Variables|Default|GetScaleScene) (Math|Rotator|MakeRotator 0.0 0.0 (.yaw (Math|Rotator|Lerp(Rotator) (Variables|Default|GetStartRotation) (Variables|Default|GetTargetRotation) _rotationspeed))) false false)
        (Development|PrintString (Utilities|String|ToString(Integer) (Variables|Default|GetRotationIndex)) true true "(R=0.000000,G=0.660000,B=1.000000,A=1.000000)" 0.0))
      (:Finished
        (Variables|Default|SetIsRotating false)))))

(fn ConstructionScript
  (|CallParentFunction)
  (Variables|Default|SetID "Package"))