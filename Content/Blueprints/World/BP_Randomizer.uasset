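; BP_Randomizer is a world actor that varies its static mesh's look and placement.
; ApplyAllVariations chains functions that randomize the mesh's relative location and per-axis scale, offset the actor's rotation, and pick a random mesh from NewMesh.
; The rotation step adds a fixed RotationOffset to every axis, leaving its random nodes unused.
; BeginPlay and the construction script are empty, so nothing here calls ApplyAllVariations; older EventGraph logic is disconnected.
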(event EventBeginPlay)

(event Collision|EventActorBeginOverlap
  (params (OtherActor :type Actor%20Object%20Reference)))

(fn ConstructionScript)

(fn RandomZ-Offset
  (bind _maxhightoffest (Variables|Default|GetMaxHightOffest))
  (bind _maxxyoffset (Variables|Default|GetMaxXYOffset))
  (bind _maxxyoffset_2 (Variables|Default|GetMaxXYOffset))
  (Transformation|SetRelativeLocation (Variables|Default|GetMesh) (Math|Vector|MakeVector (Math|Random|RandomFloatinRange (* _maxxyoffset_2 -1.0) _maxxyoffset_2) (Math|Random|RandomFloatinRange (* _maxxyoffset -1.0) _maxxyoffset) (Math|Random|RandomFloatinRange (* _maxhightoffest -1.0) _maxhightoffest)) false false)
  (return))

(fn RandomYawRollandPitch
  (bind _returnvalue (Transformation|GetActorRotation))
  (bind (_roll _pitch _yaw) (Math|Rotator|BreakRotator _returnvalue))
  (Transformation|SetActorRotation (Math|Rotator|MakeRotator (+ _roll (Variables|Default|GetRotationOffset)) (+ _pitch (Variables|Default|GetRotationOffset)) (+ _yaw (Variables|Default|GetRotationOffset)))))

(fn RandomScale
  (bind _maxrandomscalevalue (Variables|Default|GetMaxRandomScaleValue))
  (bind _minrandomscalevalue (Variables|Default|GetMinRandomScaleValue))
  (bind _returnvalue (Math|Random|RandomFloatinRange _minrandomscalevalue _maxrandomscalevalue))
  (Transformation|SetRelativeScale3D (Variables|Default|GetMesh) (Math|Vector|MakeVector _returnvalue _returnvalue _returnvalue)))

(fn SetRandomMesh
  (Components|StaticMesh|SetStaticMesh (Variables|Default|GetMesh) (.OutItem (Utilities|Array|Random (Variables|Default|GetNew%20Mesh)))))

(fn ApplyAllVariations
  (CallFunction|RandomZ-Offset)
  (CallFunction|RandomYawRollandPitch)
  (CallFunction|RandomScale)
  (CallFunction|SetRandomMesh))