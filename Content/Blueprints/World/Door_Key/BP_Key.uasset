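; BP_Key is an interactable key actor that the player picks up in the world.
; On Interact it adds its KeyID to BP_Player's CollectedKeyID, even if the player's hands are already full.
; With free hands, it becomes the HeldItemActor, attaches to the player's ItemRoot and disables its cube's shadow and collision.
; ReturnInteractStatus always reports true, and debug prints show whether the pickup reached the hand.
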(event EventBeginPlay)

(event Collision|EventActorBeginOverlap
  (params (OtherActor :type Actor%20Object%20Reference)))

(event EventTick
  (params (DeltaSeconds :type Float%20%28single-precision%29)))

(event EventInteract
  (params (Sender :type Actor%20Object%20Reference))
  (bind _asbp_player (Utilities|Casting|CastToBP_Player (Game|GetPlayerCharacter 0)))
  (Utilities|Array|Add (Variables|/Game/Blueprints/Core/BP_Player.BP_Player_C|GetCollectedKeyID _asbp_player) (Variables|Default|GetKeyID))
  (Variables|/Game/Blueprints/Core/BP_Player.BP_Player_C|GetHeldItemActor _asbp_player
    (:then
      (Development|PrintString "HandsFull" true true "(R=1.000000,G=0.000000,B=0.000000,A=1.000000)"))
    (:else
      (Variables|/Game/Blueprints/Core/BP_Player.BP_Player_C|SetHeldItemActor _asbp_player self)
      (Transformation|AttachComponentToComponent (Variables|/Game/Blueprints/Core/BP_Player.BP_Player_C|GetItemRoot _asbp_player) "None" "SnapToTarget" "SnapToTarget" "KeepRelative" true)
      (Rendering|SetCastShadow (Variables|Default|GetCube) false)
      (Collision|SetCollisionEnabled (Variables|Default|GetCube) "NoCollision")
      (Development|PrintString "ItemInHand"))))

(fn ConstructionScript)

(fn ReturnInteractStatus
  (return true))