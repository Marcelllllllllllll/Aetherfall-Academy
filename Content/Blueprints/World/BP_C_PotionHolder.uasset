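; BP_C_PotionHolder is a world slot that stores one item, presumably a potion, that the player places or picks up.
; On Interact, it checks the player's HeldItemActor against its own StoredItemActor to decide between placing and picking up.
; The item is detached and snapped to either PotionPlaceRoot or the player's ItemRoot, and the two references are swapped over.
; An occupied holder or empty-handed use of an empty holder only prints a message.
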(event EventBeginPlay)

(event Collision|EventActorBeginOverlap
  (params (OtherActor :type Actor%20Object%20Reference)))

(event EventTick
  (params (DeltaSeconds :type Float%20%28single-precision%29)))

(event EventInteract
  (params (Sender :type Actor%20Object%20Reference))
  (bind _asbp_player (Utilities|Casting|CastToBP_Player (Game|GetPlayerCharacter 0)))
  (bind _helditemactor (Variables|/Game/Blueprints/Core/BP_Player.BP_Player_C|GetHeldItemActor _asbp_player)
    (:then
      ;[0.15 0.09225 0.08853 0.5] Place
      (Variables|Default|GetStoredItemActor
        (:then
          (Development|PrintString "Holder already occupied"))
        (:else
          (Transformation|DetachFromActor _helditemactor "KeepRelative" "KeepRelative" "KeepRelative")
          (Transformation|AttachComponentToComponent _helditemactor (Variables|Default|GetPotionPlaceRoot) "None" "SnapToTarget" "SnapToTarget" "KeepRelative" true)
          (Variables|Default|SetStoredItemActor (Variables|/Game/Blueprints/Core/BP_Player.BP_Player_C|GetHeldItemActor _asbp_player))
          (Variables|/Game/Blueprints/Core/BP_Player.BP_Player_C|SetHeldItemActor _asbp_player 0))))
    (:else
      ;[0.15 0.06702 0.07225 0.5] Pickup
      (Variables|Default|GetStoredItemActor
        (:then
          (Transformation|DetachFromActor (Variables|Default|GetStoredItemActor) "KeepRelative" "KeepRelative" "KeepRelative")
          (Transformation|AttachComponentToComponent (Variables|Default|GetStoredItemActor) (Variables|/Game/Blueprints/Core/BP_Player.BP_Player_C|GetItemRoot _asbp_player) "None" "SnapToTarget" "SnapToTarget" "KeepRelative" true)
          (Variables|/Game/Blueprints/Core/BP_Player.BP_Player_C|SetHeldItemActor _asbp_player (Variables|Default|GetStoredItemActor))
          (Variables|Default|SetStoredItemActor 0))
        (:else
          (Development|PrintString "Nothing here"))))))

(fn ConstructionScript
  (|CallParentFunction))