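; Possessable puzzle pawn that the player takes control of by interacting, with empty Left/Right/Up/Down events as hooks for puzzle logic.
; Interact increments the player's CanMove counter, saves control rotation, smooth-possesses the puzzle and pushes a widget onto the main UI stack.
; IA_Move snaps input to its dominant axis to fire one direction event.
; IA_Interact possesses the player back, removes the widget and restores rotation and counter.
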(event Custom|Left)

(event Custom|Right)

(event Custom|Up)

(event Custom|Down)

(event Input|EnhancedActionEvents|EnhancedInputActionIA_Interact
  (params (ActionValue :type Boolean) (ElapsedSeconds :type Float%20%28double-precision%29) (TriggeredSeconds :type Float%20%28double-precision%29) (InputAction :type Input%20Action%20Object%20Reference :default "/Game/Inputs/IA_Interact.IA_Interact"))
  (:Started
    (Utilities|FlowControl|DoOnce false :!label _label
      (:Completed
        (Utilities|SmoothPossess (Game|GetPlayerController 0) (Variables|Default|GetAs%20BP%20Player) 1.0)
        (Class|CommonActivatableWidgetContainerBase|RemoveWidget (Utilities|ReturnMainStack (Game|GetPlayerController 0)))
        (Pawn|SetControlRotation (Game|GetPlayerController 0) (Variables|Default|GetControlRotation))
        (Math|Integer|DecrementInt (Variables|/Game/Blueprints/Core/BP_Player.BP_Player_C|GetCanMove (Variables|Default|GetAs%20BP%20Player))
          (:%20%20
            (goto _label Reset)))))))

(event Input|EnhancedActionEvents|EnhancedInputActionIA_Move
  (params (ActionValue :type Vector%202D%20Structure) (ElapsedSeconds :type Float%20%28double-precision%29) (TriggeredSeconds :type Float%20%28double-precision%29) (InputAction :type Input%20Action%20Object%20Reference :default "/Game/Inputs/IA_Move.IA_Move"))
  (bind (_x _y) (Math|Vector2D|BreakVector2D ActionValue))
  (:Started
    (if (> (Math|Float|Absolute(Float) _x) (Math|Float|Absolute(Float) _y)) ; true = left/right\nfalse = up/down
      (if (> _x 0.0)
        (CallFunction|Right)
        (else
          (CallFunction|Left)))
      (elif (> _y 0.0)
        (CallFunction|Up)
        (else
          (CallFunction|Down))))))

(event EventInteract
  (params (Sender :type Actor%20Object%20Reference))
  (bind _asbp_player (Utilities|Casting|CastToBP_Player Sender))
  (bind _output_get (Variables|Default|SetAs%20BP%20Player _asbp_player))
  (Math|Integer|IncrementInt (Variables|/Game/Blueprints/Core/BP_Player.BP_Player_C|GetCanMove _output_get)
    (:%20%20
      (Variables|Default|SetControlRotation (Pawn|GetControlRotation (Variables|Default|GetAs%20BP%20Player) :!class /Script/Engine.Pawn))
      (Utilities|SmoothPossess (Game|GetPlayerController 0) self 1.0)
      (Class|CommonActivatableWidgetContainerBase|AddWidget (Utilities|ReturnMainStack (Game|GetPlayerController 0)) (Variables|Default|GetActivatableWidget)))))

(fn ConstructionScript)

(fn ReturnInteractStatus
  (return (Variables|Default|GetIsInteractable)))