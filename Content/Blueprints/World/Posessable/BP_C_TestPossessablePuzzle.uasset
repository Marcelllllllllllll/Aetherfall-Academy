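; Test possessable puzzle actor that gives visual feedback for four directional events by changing its mesh material.
; The Left, Right, Up and Down events each set a different stock material on the mesh's first slot, with no puzzle state or solve logic.
; ReturnInteractStatus always returns false, and the construction script only calls the parent.
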(event EventLeft
  (Rendering|Material|SetMaterial (Variables|Character|GetMesh) 0 "/Engine/MapTemplates/Materials/BasicAsset01.BasicAsset01"))

(event EventRight
  (Rendering|Material|SetMaterial (Variables|Character|GetMesh) 0 "/Engine/MapTemplates/Materials/BasicAsset03.BasicAsset03"))

(event EventUp
  (Rendering|Material|SetMaterial (Variables|Character|GetMesh) 0 "/Engine/EngineDebugMaterials/BoneWeightMaterial.BoneWeightMaterial"))

(event EventDown
  (Rendering|Material|SetMaterial (Variables|Character|GetMesh) 0 "/Engine/EditorMaterials/Cascade/CASC_RenderLights_MAT.CASC_RenderLights_MAT"))

(fn ConstructionScript
  (|CallParentFunction))

(fn ReturnInteractStatus
  (return false))