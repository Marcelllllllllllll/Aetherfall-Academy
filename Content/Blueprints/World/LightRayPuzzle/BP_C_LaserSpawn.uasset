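; Laser emitter for the light ray puzzle that spawns a BP_P_Laser actor when play begins.
; On BeginPlay it stores a reference to itself and takes its display name as an ID, then spawns the laser at the Arrow component's location with the actor's rotation.
; The construction script only calls the parent version.
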(event EventBeginPlay
  (Variables|Default|SetSpawnReference self)
  (Variables|Default|SetID (Utilities|GetDisplayName self))
  (Game|SpawnActorfromClass "/Game/Blueprints/World/LightRayPuzzle/BP_P_Laser.BP_P_Laser_C" (Math|Transform|MakeTransform (Transformation|GetWorldLocation (Variables|Default|GetArrow)) (Transformation|GetActorRotation) "1.000000,1.000000,1.000000") "Undefined" "MultiplyWithRoot" 0 0 0))

(fn ConstructionScript
  (|CallParentFunction))