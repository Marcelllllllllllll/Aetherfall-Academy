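; BP_GuidingParticle is a world actor whose particle travels along a spline as a guide once a React event reports Solved.
; It activates the particle once and sets the timeline play rate from spline length and Speed, keeping travel speed independent of path length.
; The timeline update maps its value to distance along the spline to position the particle.
; An actor of a given class overlapping EndTrigger deactivates the active particle and stops the timeline.
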(event OnComponentBeginOverlap(EndTrigger)
  (params (OverlappedComponent :type Primitive%20Component%20Object%20Reference) (OtherActor :type Actor%20Object%20Reference) (OtherComp :type Primitive%20Component%20Object%20Reference) (OtherBodyIndex :type Integer) (bFromSweep :type Boolean) (SweepResult :type Hit%20Result%20Structure%20%28by%20ref%29))
  (Class|KismetSystemLibrary|IsObjectOfSoftClass OtherActor "/Game/Blueprints/Core/BP_Player.BP_Player_C"
    (:True
      (if (Components|Activation|IsActive (Variables|Default|GetParticle))
        (Utilities|FlowControl|DoOnce false
          (:Completed
            (Components|Activation|SetActive (Variables|Default|GetParticle) false false)
            (Audio|Components|Audio|Stop (Variables|Default|GetParticleTimeline))))))))

(event EventReact
  (params (Solved :type Boolean))
  (if Solved
    (Utilities|FlowControl|DoOnce false
      (:Completed
        (Components|Activation|SetActive (Variables|Default|GetParticle) true false)
        (Components|Timeline|SetPlayRate (Variables|Default|GetParticleTimeline) (/ 1.0 (/ (Spline|GetSplineLength (Variables|Default|GetSpline)) (Variables|Default|GetSpeed))))
        (Audio|Components|Audio|Play (Variables|Default|GetParticleTimeline))))))

(fn ConstructionScript)