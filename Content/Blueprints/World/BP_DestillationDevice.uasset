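; BP_DestillationDevice is an interactable world device that opens the distillation UI for the player.
; Interact calls SwitchUI on BP_HUD and passes itself as the initiating distillator, and ReturnInteractStatus always returns true.
; BeginPlay prints a red warning if no PotionHolderBP is assigned.
; Potion spawning at the holder and crystal color combination checks exist only as unconnected, unfinished logic.
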(event EventBeginPlay
  ;[0.15 0.15 0.15 0.5] Has Potionholder
  (Variables|Default|GetPotionHolderBP
    (:then)
    (:else
      (Development|PrintString "HasNoPotionHolder" true true "(R=1.000000,G=0.000000,B=0.000000,A=1.000000)" 999.0))))

(event Collision|EventActorBeginOverlap
  (params (OtherActor :type Actor%20Object%20Reference))
  ;[0.15 0.15 0.15 0.5] Has Potionholder
)

(event EventTick
  (params (DeltaSeconds :type Float%20%28single-precision%29)))

(event EventInteract
  (params (Sender :type Actor%20Object%20Reference))
  ;[0.15 0.15 0.15 0.5] Switch UI
  (bind _asbp_hud (Utilities|Casting|CastToBP_HUD (HUD|GetHUD (Game|GetPlayerController 0))))
  (Default|SwitchUI _asbp_hud true self))

(fn ConstructionScript)

(fn ReturnInteractStatus
  (return true))