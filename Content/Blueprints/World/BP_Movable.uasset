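; BP_Movable is an interactable world object that eases between its start transform and a target transform, alternating via FlipFlop and MoveComponentTo.
; Interact blocks reuse during the move, then re-enables unless set to move once; non-player senders and React skip the item check.
; With NeededID set, players need a held item, which either gets consumed to clear the requirement or triggers the move.
; The ID match is a placeholder comparing NeededID to itself.
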(event EventBeginPlay
  (Variables|Default|SetStartTransform (Transformation|GetRelativeTransform (Variables|Default|GetRoot))))

(event EventReact
  (params (Solved :type Boolean))
  ;[0 0 0 0.5] Check for ID
  (bind _isa (Utilities|FlowControl|FlipFlop)
    (:A
      _)
    (:B
      _))
  (Components|MoveComponentTo (Variables|Default|GetRoot) (.Location (Math|Transform|BreakTransform (Math|Transform|SelectTransform (Variables|Default|GetTargetTransform) (Variables|Default|GetStartTransform) _isa))) (.Rotation (Math|Transform|BreakTransform (Math|Transform|SelectTransform (Variables|Default|GetTargetTransform) (Variables|Default|GetStartTransform) _isa))) true true (Variables|Default|GetMoveDuration) true)
  (Variables|Default|GetIsMovingOnce?
    (:then)
    (:else
      (Variables|Default|SetIsInteractable true))))

(event EventInteract
  (params (Sender :type Actor%20Object%20Reference))
  (Class|KismetSystemLibrary|IsObjectOfSoftClass Sender "/Game/Blueprints/Core/BP_Player.BP_Player_C"
    (:True
      ;[0 0 0 0.5] Check for ID
      (bind _asbp_player (Utilities|Casting|CastToBP_Player Sender))
      (if (Utilities|Array|IsEmpty (Variables|Default|GetNeededID))
        (Variables|Default|SetIsInteractable false :!label _label)
        (bind _isa (Utilities|FlowControl|FlipFlop)
          (:A
            _)
          (:B
            _))
        (Components|MoveComponentTo (Variables|Default|GetRoot) (.Location (Math|Transform|BreakTransform (Math|Transform|SelectTransform (Variables|Default|GetTargetTransform) (Variables|Default|GetStartTransform) _isa))) (.Rotation (Math|Transform|BreakTransform (Math|Transform|SelectTransform (Variables|Default|GetTargetTransform) (Variables|Default|GetStartTransform) _isa))) true true (Variables|Default|GetMoveDuration) true)
        (Variables|Default|GetIsMovingOnce?
          (:then)
          (:else
            (Variables|Default|SetIsInteractable true)))
        (else
          (Utilities|IsValid (Variables|/Game/Blueprints/Core/BP_Player.BP_Player_C|GetHeldItemActor _asbp_player)
            (:Is%20Valid
              (if (Utilities|Enum|Equal(Enum) (Variables|Default|GetNeededID) (Variables|Default|GetNeededID))
                (Variables|Default|GetDestroyItem
                  (:then
                    (Variables|Default|SetNeededID "")
                    (Actor|DestroyActor (Variables|/Game/Blueprints/Core/BP_Player.BP_Player_C|GetHeldItemActor _asbp_player))
                    (Variables|/Game/Blueprints/Core/BP_Player.BP_Player_C|SetHeldItemActor _asbp_player 0))
                  (:else
                    (goto _label)))))
            (:Is%20Not%20Valid)))))
    (:False
      (goto _label))))

(fn ConstructionScript)

(fn ReturnInteractStatus
  (return (Variables|Default|GetIsInteractable)))