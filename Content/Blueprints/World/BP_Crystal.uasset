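; BP_Crystal is an interactable world pickup that comes in red, blue or green.
; The construction script applies the material matching CrystalColor, and BeginPlay creates a dynamic material instance from it on the mesh.
; Interact passes the color to BP_Player through AddCrystalColor and destroys the crystal, while ReturnInteractStatus exposes the IsInteractable flag.
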(event EventBeginPlay
  (switch Utilities|FlowControl|Switch|SwitchonE_CrystalColor (Variables|Default|GetCrystalColor)
    (:NewEnumerator0
      (Rendering|Material|CreateDynamicMaterialInstance (Variables|Default|GetStaticMesh) 0 "/Game/Materials/World/MI_CrystalRed.MI_CrystalRed" "None" :!class /Script/Engine.PrimitiveComponent))
    (:NewEnumerator1
      (Rendering|Material|CreateDynamicMaterialInstance (Variables|Default|GetStaticMesh) 0 "/Game/Materials/World/MI_CrystalBlue.MI_CrystalBlue" "None" :!class /Script/Engine.PrimitiveComponent))
    (:NewEnumerator2
      (Rendering|Material|CreateDynamicMaterialInstance (Variables|Default|GetStaticMesh) 0 "/Game/Materials/World/MI_CrystalGreen.MI_CrystalGreen" "None" :!class /Script/Engine.PrimitiveComponent))))

(event Collision|EventActorBeginOverlap
  (params (OtherActor :type Actor%20Object%20Reference)))

(event EventTick
  (params (DeltaSeconds :type Float%20%28single-precision%29)))

(event EventInteract
  (params (Sender :type Actor%20Object%20Reference))
  (bind _asbp_player (Utilities|Casting|CastToBP_Player (Game|GetPlayerCharacter 0)))
  (Default|AddCrystalColor _asbp_player (Variables|Default|GetCrystalColor))
  (Actor|DestroyActor))

(fn ConstructionScript
  (Rendering|Material|SetMaterial (Variables|Default|GetStaticMesh) 0 (Utilities|Select :Index (Variables|Default|GetCrystalColor) :NewEnumerator0 "/Game/Materials/World/MI_CrystalRed.MI_CrystalRed" :NewEnumerator1 "/Game/Materials/World/MI_CrystalBlue.MI_CrystalBlue" :NewEnumerator2 "/Game/Materials/World/MI_CrystalGreen.MI_CrystalGreen")))

(fn ReturnInteractStatus
  (return (Variables|Default|GetIsInteractable)))