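; BP_HighJumpPotion is an interactable world object that temporarily lowers the player's gravity, giving higher jumps.
; On Interact, it casts the sender to BP_Player, sets the CharacterMovement gravity scale to a lower value, then restores a hardcoded higher value after a short delay, printing each change.
; It always reports a true interact status, clears its ID in the construction script, and is not destroyed on use.
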(event EventInteract
  (params (Sender :type Actor%20Object%20Reference))
  (bind _asbp_player (Utilities|Casting|CastToBP_Player Sender))
  (Variables|/Script/Engine.CharacterMovementComponent|SetGravityScale (Variables|/Script/Engine.Character|GetCharacterMovement _asbp_player) 1.0)
  (Development|PrintString "Gravity =1")
  (Utilities|FlowControl|Delay 3.0)
  (Variables|/Script/Engine.CharacterMovementComponent|SetGravityScale (Variables|/Script/Engine.Character|GetCharacterMovement _asbp_player) 3.0)
  (Development|PrintString "Gravity =3"))

(fn ConstructionScript
  (|CallParentFunction)
  (Variables|Default|SetID ""))

(fn ReturnInteractStatus
  (return true))