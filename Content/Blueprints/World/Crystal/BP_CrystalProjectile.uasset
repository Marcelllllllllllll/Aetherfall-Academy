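; BP_CrystalProjectile is a crystal projectile that launches itself when play begins.
; On BeginPlay it switches on CrystalColor to apply a dynamic material instance of the red, blue or green crystal material to its static mesh.
; It then applies ThrowForce to the mesh as a mass-dependent physics impulse; the file shows no hit handling.
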(event EventBeginPlay
  (switch Utilities|FlowControl|Switch|SwitchonE_CrystalColor (Variables|Default|GetCrystalColor)
    (:NewEnumerator0
      (Rendering|Material|CreateDynamicMaterialInstance (Variables|Default|GetStaticMesh) 0 "/Game/Materials/World/MI_CrystalRed.MI_CrystalRed" "None" :!class /Script/Engine.PrimitiveComponent))
    (:NewEnumerator1
      (Rendering|Material|CreateDynamicMaterialInstance (Variables|Default|GetStaticMesh) 0 "/Game/Materials/World/MI_CrystalBlue.MI_CrystalBlue" "None" :!class /Script/Engine.PrimitiveComponent))
    (:NewEnumerator2
      (Rendering|Material|CreateDynamicMaterialInstance (Variables|Default|GetStaticMesh) 0 "/Game/Materials/World/MI_CrystalGreen.MI_CrystalGreen" "None" :!class /Script/Engine.PrimitiveComponent)))
  (Physics|AddImpulse (Variables|Default|GetStaticMesh) (Variables|Default|GetThrowForce) "None" false))

(fn ConstructionScript)