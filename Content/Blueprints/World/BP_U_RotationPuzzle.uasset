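; BP_U_RotationPuzzle is an interactable puzzle piece that rotates through preset orientations and counts as solved at one designated position.
; Each Interact advances the index through RotationPoints, wrapping to the start, and snaps RotationScene to that rotation.
; It updates Solved and notifies ActorToReact through ReactMessage when solved or moved off the solution.
; The construction script applies the starting rotation, and getters expose the interactable and solved states.
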(event EventInteract
  (params (Sender :type Actor%20Object%20Reference))
  (Variables|Default|SetCurrentPositionIndex (Math|Integer|SelectInt 0 (+ (Variables|Default|GetCurrentPositionIndex) 1) (> (+ (Variables|Default|GetCurrentPositionIndex) 1) (Utilities|Array|LastIndex (Variables|Default|GetRotationPoints)))))
  (Transformation|SetRelativeRotation (Variables|Default|GetRotationScene) (Utilities|Array|Get(acopy) (Variables|Default|GetRotationPoints) (Variables|Default|GetCurrentPositionIndex)) false false)
  (if (== (Variables|Default|GetCurrentPositionIndex) (Variables|Default|GetSolvedPositionIndex))
    (Variables|Default|SetSolved true)
    (Class|BPIReact|React(Message) (Variables|Default|GetActorToReact) true)
    (else
      (Variables|Default|GetSolved
        (:then
          (Variables|Default|SetSolved false)
          (Class|BPIReact|React(Message) (Variables|Default|GetActorToReact) false))
        (:else)))))

(event EventSetInteractStatus
  (params (IsInteractable :type Boolean))
  (Variables|Default|SetIsInteractable IsInteractable))

(fn ConstructionScript
  (Transformation|SetRelativeRotation (Variables|Default|GetRotationScene) (Utilities|Array|Get(acopy) (Variables|Default|GetRotationPoints) (Variables|Default|GetCurrentPositionIndex)) true false))

(fn ReturnInteractStatus
  (return (Variables|Default|GetIsInteractable)))

(fn ReturnSolvedStatus
  (return (Variables|Default|GetSolved)))