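; Potion actor that the player can pick up, with a color variant or an empty glass, identified as "PotionGlass".
; On BeginPlay, PotionColor sets a dynamic glass material and a colored material, or swaps in the empty glass mesh.
; Interact attaches the potion to the player's ItemRoot when HeldItemActor is invalid, without setting that variable here.
; The detach and parent Interact calls are left unconnected.
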(event EventBeginPlay
  (switch Utilities|FlowControl|Switch|SwitchonE_PotionColor (Variables|Default|GetPotionColor)
    (:NewEnumerator0
      (Rendering|Material|CreateDynamicMaterialInstance (Variables|Character|GetMesh) 0 "/Game/Materials/World/MI_PotionGlass.MI_PotionGlass" "None" :!class /Script/Engine.PrimitiveComponent)
      (Rendering|Material|SetMaterial (Variables|Character|GetMesh) 1 "/Game/Materials/World/MI_PotionLightBlue.MI_PotionLightBlue"))
    (:NewEnumerator1
      (Rendering|Material|CreateDynamicMaterialInstance (Variables|Character|GetMesh) 0 "/Game/Materials/World/MI_PotionGlass.MI_PotionGlass" "None" :!class /Script/Engine.PrimitiveComponent)
      (Rendering|Material|SetMaterial (Variables|Character|GetMesh) 1 "/Game/Materials/World/MI_PotionPink.MI_PotionPink"))
    (:NewEnumerator2
      (Rendering|Material|CreateDynamicMaterialInstance (Variables|Character|GetMesh) 0 "/Game/Materials/World/MI_PotionGlass.MI_PotionGlass" "None" :!class /Script/Engine.PrimitiveComponent)
      (Rendering|Material|SetMaterial (Variables|Character|GetMesh) 1 "/Game/Materials/World/MI_PotionYellow.MI_PotionYellow"))
    (:NewEnumerator3
      (Components|StaticMesh|SetStaticMesh (Variables|Character|GetMesh) "/Game/3D/HighBlockoutMesh/Potion/PotionGlassEmpty.PotionGlassEmpty"))))

(event Collision|EventActorBeginOverlap
  (params (OtherActor :type Actor%20Object%20Reference)))

(event EventTick
  (params (DeltaSeconds :type Float%20%28single-precision%29)))

(event EventInteract
  (params (Sender :type Actor%20Object%20Reference))
  (bind _asbp_player (Utilities|Casting|CastToBP_Player (Game|GetPlayerCharacter 0)))
  (Utilities|IsValid (Variables|/Game/Blueprints/Core/BP_Player.BP_Player_C|GetHeldItemActor _asbp_player)
    (:Is%20Not%20Valid
      (Transformation|AttachComponentToComponent self (Variables|/Game/Blueprints/Core/BP_Player.BP_Player_C|GetItemRoot _asbp_player) "None" "SnapToTarget" "SnapToTarget" "KeepRelative" true)
      (Development|PrintString "ItemInHand"))))

(fn ConstructionScript
  (|CallParentFunction)
  (Variables|Default|SetID "PotionGlass"))