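; BP_CutscenePlayer plays a level sequence when it receives a solved React, then forwards the reaction to another actor.
; The player's CanMove counter increments during playback and decrements when the cutscene ends, while ActorToReact receives its message after ReactDelay.
; A PlayOnce check routes through DoOnceWithAfter, so later solves skip the cutscene and react immediately.
; An unsolved React forwards false without playback.
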(event Custom|OnCutsceneEnd
  (bind _playerref (Variables|Default|GetPlayerRef)
    (:then
      (Math|Integer|DecrementInt (Variables|/Game/Blueprints/Core/BP_Player.BP_Player_C|GetCanMove _playerref)))
    (:else)))

(event EventReact
  (params (Solved :type Boolean))
  (bind _cutscenetoplay (Variables|Default|GetCutsceneToPlay))
  (bind _sequenceplayer (Variables|/Script/LevelSequence.LevelSequenceActor|GetSequencePlayer _cutscenetoplay))
  (if Solved
    (Variables|Default|GetPlayOnce
      (:then
        (Utilities|DoOncewithAfter
          (:Once
            (Utilities|FlowControl|Sequence :!label _label
              (:then_0
                (Variables|Default|GetPlayerRef
                  (:then
                    _)
                  (:else
                    (bind _returnvalue (Actor|GetActorOfClass "/Game/Blueprints/Core/BP_Player.BP_Player_C"))
                    (Variables|Default|SetPlayerRef _returnvalue)))
                (Math|Integer|IncrementInt (Variables|/Game/Blueprints/Core/BP_Player.BP_Player_C|GetCanMove (Variables|Default|GetPlayerRef))
                  (:%20%20
                    (Sequencer|Player|Play _sequenceplayer :!class /Script/MovieScene.MovieSceneSequencePlayer)
                    (EventDispatchers|BindEventtoOnFinished _sequenceplayer (delegate Custom|OnCutsceneEnd)))))
              (:then_1
                (Utilities|FlowControl|Delay (Variables|Default|GetReactDelay))
                (Class|BPIReact|React(Message) (Variables|Default|GetActorToReact) true))))
          (:After
            (Class|BPIReact|React(Message) (Variables|Default|GetActorToReact) true))))
      (:else
        (goto _label)))
    (else
      (Class|BPIReact|React(Message) (Variables|Default|GetActorToReact) false))))

(fn ConstructionScript)