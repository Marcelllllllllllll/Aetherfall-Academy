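; BP_CollectableSocket is an interactable world socket that receives the item the player is holding.
; On Interact from a BP_Player sender, it caches the player reference and attaches the held item actor to its CollectableScene component, snapping location, rotation and scale.
; An IsInteractable flag is exposed through set and return functions, though Interact itself does not check it.
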(event EventBeginPlay)

(event EventInteract
  (params (Sender :type Actor%20Object%20Reference))
  (Class|KismetSystemLibrary|IsObjectOfSoftClass Sender "/Game/Blueprints/Core/BP_Player.BP_Player_C"
    (:True
      (Variables|Default|GetPlayerRef
        (:then
          _)
        (:else
          (bind _asbp_player (Utilities|Casting|CastToBP_Player Sender))
          (Variables|Default|SetPlayerRef _asbp_player)))
      (bind _helditemactor (Variables|/Game/Blueprints/Core/BP_Player.BP_Player_C|GetHeldItemActor (Variables|Default|GetPlayerRef))
        (:then
          (Transformation|AttachComponentToComponent _helditemactor (Variables|Default|GetCollectableScene) "None" "SnapToTarget" "SnapToTarget" "SnapToTarget" true))
        (:else)))))

(event EventSetInteractStatus
  (params (IsInteractable :type Boolean))
  (Variables|Default|SetIsInteractable IsInteractable))

(fn ConstructionScript)

(fn ReturnInteractStatus
  (return (Variables|Default|GetIsInteractable)))