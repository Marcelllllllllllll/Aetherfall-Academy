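; Interactable rotation potion that turns a referenced room around its vertical axis when BP_Player interacts with it.
; A timeline drives the room root's relative yaw, scaled by RotationValue, and plays a 2D sound on every update.
; On finish it fires RotationFinished, which calls Play on the timeline again.
; The construction script sets the item ID, and interact status always returns true.
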(event Custom|RotationFinished
  (bind _rotation (Timeline|RotationTimeline Play)
    (:Update
      (Transformation|SetRelativeRotation (Variables|/Game/Blueprints/World/BP_Room.BP_Room_C|GetDefaultRoot (Variables|Default|GetRoomRef)) (Math|Rotator|MakeRotator 0.0 0.0 (* _rotation (Variables|Default|GetRotationValue))) false false)
      (Audio|PlaySound2D 0 1.0 1.0 0.0 0 0))
    (:Finished
      (CallFunction|RotationFinished))))

(event EventBeginPlay)

(event Collision|EventActorBeginOverlap
  (params (OtherActor :type Actor%20Object%20Reference)))

(event EventTick
  (params (DeltaSeconds :type Float%20%28single-precision%29)))

(event EventInteract
  (params (Sender :type Actor%20Object%20Reference))
  (bind _roomref (Variables|Default|GetRoomRef))
  (Utilities|Casting|CastToBP_Player Sender)
  (Utilities|IsValid _roomref
    (:Is%20Valid
      (bind _rotation (Timeline|RotationTimeline Play)
        (:Update
          (Transformation|SetRelativeRotation (Variables|/Game/Blueprints/World/BP_Room.BP_Room_C|GetDefaultRoot _roomref) (Math|Rotator|MakeRotator 0.0 0.0 (* _rotation (Variables|Default|GetRotationValue))) false false)
          (Audio|PlaySound2D 0 1.0 1.0 0.0 0 0))
        (:Finished
          (CallFunction|RotationFinished))))))

(fn ConstructionScript
  (|CallParentFunction)
  (Variables|Default|SetID "RotationPotion"))

(fn ReturnInteractStatus
  (return true))